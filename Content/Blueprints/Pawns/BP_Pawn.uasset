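; Player character pawn with Enhanced Input movement, camera look, sprint, delayed standstill jump animation, self-kill, and an optional socket-attached weapon built at construction.
; Hits damage the other actor.
; Any damage triggers a one-time death: movement stops, the mesh ragdolls upward, the capsule switches to Spectator collision, and the pawn expires.
; Tick detects floor changes and sends BI_Floor off/on notifications to the previous and current floor actors.
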(event EventTick
  (params (DeltaSeconds :type Float%20%28single-precision%29))
  (bind (_cullentfloor _returnvalue) (|LastFloorIsNotSameCurrentFloor))
  (if _returnvalue
    (Utilities|FlowControl|Sequence
      (:then_0
        (bind _asbi_floor (Utilities|Casting|CastToBI_Floor (Variables|Default|GetLastFloor)))
        (Default|OnPawnOff _asbi_floor self))
      (:then_1
        (bind _asbi_floor_2 (Utilities|Casting|CastToBI_Floor _cullentfloor))
        (Default|OnPawnon _asbi_floor_2 self))
      (:then_2
        (Variables|Default|SetLastFloor _cullentfloor)))))

(event Game|Damage|EventAnyDamage
  (params (Damage :type Float%20%28single-precision%29) (DamageType :type Damage%20Type%20Object%20Reference) (InstigatedBy :type Controller%20Object%20Reference) (DamageCauser :type Actor%20Object%20Reference))
  (bind _mesh (Variables|Character|GetMesh))
  ;[1 1 1] 自爆
  (Utilities|FlowControl|DoOnce false
    (:Completed
      (Development|PrintString "I Will be Back")
      (Pawn|Components|CharacterMovement|DisableMovement (Variables|Character|GetCharacterMovement))
      (Actor|SetLifeSpan 5.0) ; 5秒後に消滅
      (Utilities|FlowControl|Sequence
        (:then_0
          ;[1 1 1] ラグドールになる
          (Collision|SetCollisionProfileName _mesh "Ragdoll" true :!class /Script/Engine.PrimitiveComponent)
          (Class|SkeletalMeshComponent|SetAllBodiesSimulatePhysics _mesh true)
          (Class|SkeletalMeshComponent|AddImpulsetoAllBodiesBelow _mesh "0.000000,0.000000,500.000000" "None" true true) ; 上に飛ばす
        )
        (:then_1
          ;[1 1 1] カプセルの当たり判定を無視する (p517 通過ノ試練)
          (Collision|SetCollisionProfileName (Variables|Collision|GetCapsuleComponent) "Spectator" true :!class /Script/Engine.PrimitiveComponent))))))

(event Collision|EventHit
  (params (MyComp :type Primitive%20Component%20Object%20Reference) (Other :type Actor%20Object%20Reference) (OtherComp :type Primitive%20Component%20Object%20Reference) (bSelfMoved :type Boolean) (HitLocation :type Vector :default "0, 0, 0") (HitNormal :type Vector :default "0, 0, 0") (NormalImpulse :type Vector :default "0, 0, 0") (Hit :type Hit%20Result%20Structure%20%28by%20ref%29))
  ;[1 1 1] 当たった相手にダメージを追加
  (Game|Damage|ApplyDamage Other 1.0 0 self))

(event EventOnJumped
  ;[1 1 1] ジャンプの開始通知 (p450)
  (Default|CallOnPawnJumped))

(event Input|EnhancedActionEvents|EnhancedInputActionIA_Jump
  (params (ActionValue :type Boolean) (ElapsedSeconds :type Float%20%28double-precision%29) (TriggeredSeconds :type Float%20%28double-precision%29) (InputAction :type Input%20Action%20Object%20Reference :default "/Game/Inputs/IA_Jump.IA_Jump"))
  ;[1 1 1] ジャンプ
  (:Triggered
    (if (Character|CanJump)
      (if (>= (Math|Vector|VectorLengthXY (Transformation|GetVelocity)) 1e+01)
        _
        (else
          (Class|AnimInstance|RequestTransitionEvent (Components|SkeletalMesh|GetAnimInstance (Variables|Character|GetMesh)) "StartJump" 0.1 "Shared" "Append")
          (Utilities|FlowControl|Delay 0.2)))
      (Character|Jump))))

(event Input|EnhancedActionEvents|EnhancedInputActionIA_Sprint
  (params (ActionValue :type Boolean) (ElapsedSeconds :type Float%20%28double-precision%29) (TriggeredSeconds :type Float%20%28double-precision%29) (InputAction :type Input%20Action%20Object%20Reference :default "/Game/Inputs/IA_Sprint.IA_Sprint"))
  ;[1 1 1] ダッシュ
  (:Triggered
    (CallFunction|BeginSprint))
  (:Completed
    (CallFunction|EndSprint)))

(event Input|EnhancedActionEvents|EnhancedInputActionIA_FoceKill
  (params (ActionValue :type Boolean) (ElapsedSeconds :type Float%20%28double-precision%29) (TriggeredSeconds :type Float%20%28double-precision%29) (InputAction :type Input%20Action%20Object%20Reference :default "/Game/Inputs/IA_FoceKill.IA_FoceKill"))
  (bind _self self)
  ;[1 1 1] 自爆
  (:Triggered
    (Game|Damage|ApplyDamage _self 1.0 0 _self) ; 自分自身にダメージを適用
  ))

(event Input|EnhancedActionEvents|EnhancedInputActionIA_Look
  (params (ActionValue :type Vector%202D%20Structure) (ElapsedSeconds :type Float%20%28double-precision%29) (TriggeredSeconds :type Float%20%28double-precision%29) (InputAction :type Input%20Action%20Object%20Reference :default "/Game/Inputs/IA_Look.IA_Look"))
  (bind (_x _y) (Math|Vector2D|BreakVector2D ActionValue))
  ;[1 1 1] カメラ操作
  (:Triggered
    (Pawn|Input|AddControllerYawInput _x)
    (Pawn|Input|AddControllerPitchInput _y)))

(event Input|EnhancedActionEvents|EnhancedInputActionIA_Move
  (params (ActionValue :type Vector%202D%20Structure) (ElapsedSeconds :type Float%20%28double-precision%29) (TriggeredSeconds :type Float%20%28double-precision%29) (InputAction :type Input%20Action%20Object%20Reference :default "/Game/Inputs/IA_Move.IA_Move"))
  (bind (_x _y) (Math|Vector2D|BreakVector2D ActionValue))
  ;[1 1 1] 移動
  (:Triggered
    (Pawn|Input|AddMovementInput (|CameraForwardVector) _y false) ; 前後移動
    (Pawn|Input|AddMovementInput (Math|Vector|GetRightVector (Variables|Default|GetCamera)) _x false) ; 左右移動
  ))

(fn ConstructionScript
  ;[1 1 1] Static Mesh Componentの追加 (p549)
  (Utilities|IsValid (Variables|Default|GetWeaponMeshAsset)
    (:Is%20Valid
      (bind _returnvalue (AddComponent|AddStaticMeshComponent true))
      (bind _output_get (LocalVariables|SetWeaponMesh _returnvalue))
      ;[1 1 1] 武器を持つ
      (Components|StaticMesh|SetStaticMesh _output_get (Variables|Default|GetWeaponMeshAsset))
      (Transformation|AttachComponentToComponent (LocalVariables|GetWeaponMesh) (Variables|Character|GetMesh) "weapon_r" "SnapToTarget" "SnapToTarget" "SnapToTarget" true))))

(fn BeginSprint
  (if (Variables|Default|GetIsSprinting) ; スプリント状態を確認
    (return false) ; 失敗
    (else
      (Variables|/Script/Engine.CharacterMovementComponent|SetMaxWalkSpeed (Variables|Character|GetCharacterMovement) 2e+02) ; スプリント速度を設定
      (Variables|Default|SetIsSprinting true) ; スプリント状態になった
      (return true))))

(fn EndSprint
  (if (Variables|Default|GetIsSprinting)
    (Variables|/Script/Engine.CharacterMovementComponent|SetMaxWalkSpeed (Variables|Character|GetCharacterMovement) 75.0) ; スプリント速度を設定
    (Variables|Default|SetIsSprinting false) ; Sprint状態を戻す
    (return true)
    (else
      (return false))))

(fn GetIsSprinting
  (return (Variables|Default|GetIsSprinting)))

(fn GetCullentFloor
  (return (.HitActor (Collision|BreakHitResult (.HitResult (Utilities|Struct|BreakFindFloorResult (Variables|/Script/Engine.CharacterMovementComponent|GetCurrentFloor (Variables|Character|GetCharacterMovement))))))))