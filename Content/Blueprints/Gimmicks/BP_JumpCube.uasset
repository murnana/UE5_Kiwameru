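; BP_JumpCube is a gimmick cube that moves up or down when a pawn on it jumps.
; Pawn on/off events swap the cube's grid material and bind or unbind CubeMove to the pawn's jump event.
; CubeMove flip-flops a timeline forward and back toward DestTransform, applying per-frame transform deltas to the actor's current transform.
; A conditional Reset re-enters the same flip-flop.
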(event EventOnPawnOff
  (params (Pawn :type Pawn%20Object%20Reference))
  (|RestoreColorChange)
  (bind _asbp_pawn (Utilities|Casting|CastToBP_Pawn Pawn))
  (EventDispatchers|UnbindEventfromOnPawnJumped _asbp_pawn (|CubeMove)))

(event EventOnPawnon
  (params (Pawn :type Pawn%20Object%20Reference))
  (|ColorChange)
  (bind _asbp_pawn (Utilities|Casting|CastToBP_Pawn Pawn))
  (EventDispatchers|AssignOnPawnJumped _asbp_pawn (|CubeMove)))

(fn ConstructionScript)

(event Custom|Toggle
  ;[1 1 1] リセット動作
  (bind _isa (Utilities|FlowControl|FlipFlop)
    (:A
      ;[1 1 1] Cubeの上下動
      (bind _alpha (Timeline|CubeTL Play) ; キューブの上昇
        (:Update
          (Transformation|SetActorTransform (Math|Transform|ComposeTransforms (Math|Transform|ComposeTransforms (Math|Transform|Lerp(Transform) (Variables|Default|GetIdentity) (Variables|Default|GetDestTransform) _alpha) (Math|Transform|InvertTransform (Variables|Default|GetDummyCube))) (Transformation|GetActorTransform)))
          (Variables|Default|SetDummyCube (Math|Transform|Lerp(Transform) (Variables|Default|GetIdentity) (Variables|Default|GetDestTransform) _alpha)))))
    (:B
      (Timeline|CubeTL Reverse))))

(event Custom|Reset
  ;[1 1 1] リセット動作
  (if (stale _isa)
    (bind _isa (Utilities|FlowControl|FlipFlop)
      (:A
        ;[1 1 1] Cubeの上下動
        (bind _alpha (Timeline|CubeTL Play) ; キューブの上昇
          (:Update
            (Transformation|SetActorTransform (Math|Transform|ComposeTransforms (Math|Transform|ComposeTransforms (Math|Transform|Lerp(Transform) (Variables|Default|GetIdentity) (Variables|Default|GetDestTransform) _alpha) (Math|Transform|InvertTransform (Variables|Default|GetDummyCube))) (Transformation|GetActorTransform)))
            (Variables|Default|SetDummyCube (Math|Transform|Lerp(Transform) (Variables|Default|GetIdentity) (Variables|Default|GetDestTransform) _alpha)))))
      (:B
        (Timeline|CubeTL Reverse)))))