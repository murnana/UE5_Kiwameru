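; BP_Bullet is a physics-driven glowing projectile that deals damage on its first hit.
; BeginPlay launches the mesh forward with a velocity-change impulse, and Tick applies an upward acceleration offsetting most of standard gravity for a flatter arc.
; The first hit applies damage, stops that lift, ignores further Pawn collisions and turns off the glow.
; The Construction Script creates the dynamic material that carries the configurable bullet color.
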(event Collision|EventHit
  (params (MyComp :type Primitive%20Component%20Object%20Reference) (Other :type Actor%20Object%20Reference) (OtherComp :type Primitive%20Component%20Object%20Reference) (bSelfMoved :type Boolean) (HitLocation :type Vector :default "0, 0, 0") (HitNormal :type Vector :default "0, 0, 0") (NormalImpulse :type Vector :default "0, 0, 0") (Hit :type Hit%20Result%20Structure%20%28by%20ref%29))
  (Utilities|FlowControl|DoOnce false
    (:Completed
      (Game|Damage|ApplyDamage Other 1.0 0 self)
      (Actor|Tick|SetActorTickEnabled false) ; 揚力を切る
      ;[1 1 1] 対ポーンヒットの無効化
      (Collision|SetCollisionResponsetoChannel (Variables|Debug|GetStaticMeshComponent) "ECC_Pawn" "ECR_Ignore")
      ;[1 1 1] 光を失う (p676)
      (Rendering|Material|SetScalarParameterValue (Variables|Default|GetBullet%20MI) "Emissive Intensity" 0.0 :!class /Script/Engine.MaterialInstanceDynamic))))

(event EventBeginPlay
  ;[1 1 1] 弾丸を物理演算で発射 (p505)
  (Physics|AddImpulse (Variables|Debug|GetStaticMeshComponent) (* (Transformation|GetActorForwardVector) (Variables|Default|GetBulletInitalSpeed)) "None" true) ; 弾丸を初速度ではじき出す
)

(event EventTick
  (params (DeltaSeconds :type Float%20%28single-precision%29))
  ;[1 1 1] 揚力を聞かせる (p506)
  (Physics|AddForce (Variables|Debug|GetStaticMeshComponent) (Math|Vector|Lerp(Vector) "0.000000,0.000000,980.000000" "0, 0, 0" 0.2) "None" true))

(fn ConstructionScript
  (bind _returnvalue (Rendering|Material|CreateDynamicMaterialInstance (Variables|Debug|GetStaticMeshComponent) 0 "/Game/Props/Materials/MI_Bullet.MI_Bullet" "None" :!class /Script/Engine.PrimitiveComponent))
  (bind _output_get (Variables|Default|SetBullet%20MI _returnvalue))
  (Rendering|Material|SetVectorParameterValue _output_get "Emissive Color" (Variables|Default|GetBulletColor) :!class /Script/Engine.MaterialInstanceDynamic))