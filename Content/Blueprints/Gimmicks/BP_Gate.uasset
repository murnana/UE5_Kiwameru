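; BP_Gate is a double-door gate gimmick that slides open and shut through its Open and Close events.
; Open plays the GateTL timeline, while Close runs a separately named timeline in reverse from its end.
; Each timeline's RightGate vector sets the right door's relative location, and the same vector with Y negated mirrors it onto the left door.
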(event Custom|Close
  ;[1 1 1] 扉を開く
  (bind _rightgate (Timeline|タイムライン ReverseFromEnd)
    (:Update
      (Transformation|SetRelativeLocation (Variables|Default|GetSM_Gate_L) (* _rightgate "1.000000,-1.000000,1.000000") false false) ; 左の戸の相対位置指定
      (Transformation|SetRelativeLocation (Variables|Default|GetSM_Gate_R) _rightgate false false) ; 右の戸の相対位置指定
    )))

(event Custom|Open
  ;[1 1 1] 扉を開く
  (bind _rightgate (Timeline|GateTL Play)
    (:Update
      (Transformation|SetRelativeLocation (Variables|Default|GetSM_Gate_L) (* _rightgate "1.000000,-1.000000,1.000000") false false) ; 左の戸の相対位置指定
      (Transformation|SetRelativeLocation (Variables|Default|GetSM_Gate_R) _rightgate false false) ; 右の戸の相対位置指定
    )))

(event EventBeginPlay)

(event Collision|EventActorBeginOverlap
  (params (OtherActor :type Actor%20Object%20Reference)))

(event EventTick
  (params (DeltaSeconds :type Float%20%28single-precision%29)))

(fn ConstructionScript)