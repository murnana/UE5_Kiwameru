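; BP_Scroll is a scroll pickup that a Character cannot obtain while falling.
; It overrides CanBeObtained, combining a not-falling check on the pawn's CharacterMovement with the parent's result.
; A helper macro casts the pawn to Character to get that component; when the cast fails, the parent's check alone decides.
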(fn ConstructionScript)

(fn CanbeObtained
  (params (Pawn :type Pawn%20Object%20Reference) (PlayerController :type Player%20Controller%20Object%20Reference))
  (bind _returnvalue (|CallParentFunction Pawn PlayerController))
  (bind _charactermovement (|TryGetCharacterMovement Pawn)
    (:then
      (return (and (|IsNotFalling _charactermovement) _returnvalue)))
    (:CastFailed
      (return _returnvalue))))