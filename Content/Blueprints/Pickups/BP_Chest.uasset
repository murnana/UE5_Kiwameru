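; BP_Chest is a treasure chest pickup that bursts into a shower of coins when obtained.
; Its ObstainedImpl event loops to spawn tossed BP_Coin actors at the chest's transform.
; Each coin's launch velocity is the TossVelocity vector rotated by a fixed pitch and random yaw, scattering the coins around the chest.
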(event EventBeginPlay
  (|CallParentFunction) ; このノードは無効になっているため呼び出せません。\n機能をビルドするにはピンをドラッグしてください。
)

(event Collision|EventActorBeginOverlap
  (params (OtherActor :type Actor%20Object%20Reference))
  (|CallParentFunction OtherActor) ; このノードは無効になっているため呼び出せません。\n機能をビルドするにはピンをドラッグしてください。
)

(event EventTick
  (params (DeltaSeconds :type Float%20%28single-precision%29))
  (|CallParentFunction DeltaSeconds) ; このノードは無効になっているため呼び出せません。\n機能をビルドするにはピンをドラッグしてください。
)

(event EventObstainedImpl
  (params (Pawn :type Pawn%20Object%20Reference) (PlayerController :type Player%20Controller%20Object%20Reference))
  ;[1 1 1] 宝箱からコインをスポーン
  (for _index (range 0 10) ; Spawnを10回反復実行
    (Game|SpawnActorfromClass "/Game/Blueprints/Pickups/BP_Coin.BP_Coin_C" (Transformation|GetActorTransform) "Undefined" 0 true (Math|Transform|TransformDirection (Math|Transform|MakeTransform "0, 0, 0" (Math|Rotator|MakeRotator 0.0 2e+01 (Math|Random|RandomFloatinRange 0.0 3.6e+02))) (Variables|Default|GetToss%20Velocity)) 1e+01 0)))

(fn ConstructionScript
  (|CallParentFunction))