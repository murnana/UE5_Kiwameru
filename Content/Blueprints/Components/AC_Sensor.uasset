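; AC_Sensor is a sensor component that finds pawns inside a view cone defined by sight length and angle, for deciding when to fire.
; CheckSensor sweeps a box trace along the forward ray, sized by the tangent of the half angle to cover the cone.
; CanSeeActor filters hits with a dot-product angle test and a line trace for occlusion.
; It returns visible actors and whether any exist, with debug drawing.
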(fn CheckSensor
  (bind (_start _end _rotation _location _returnvalue) (|GetMuzzleRay))
  (bind _sightangle (Variables|Default|GetSightAngle))
  (bind _returnactors (LocalVariables|GetReturnActors))
  (bind _sightlength (Variables|Default|GetSightLength))
  (bind _returnvalue_2 (* _sightangle 0.5))
  (bind _returnvalue_3 (Math|Trig|Tan(Degrees) _returnvalue_2))
  (bind _returnvalue_4 (* _sightlength _returnvalue_3))
  ;[1 1 1] センサー内にいるポーンを探す
  (bind _outhits (Class|KismetSystemLibrary|BoxTraceMulti _start _end (Math|Vector|MakeVector 0.0 _returnvalue_4 _returnvalue_4) _rotation "TraceTypeQuery4" false 0 "ForOneFrame" true))
  (for _array_element _outhits
    ;[1 1 1] ポーンが射程にいたら、射撃開始 (p531)
    (bind _returnvalue_5 (CallFunction|CanSeeActor (.HitActor (Collision|BreakHitResult _array_element))))
    (if _returnvalue_5
      (Utilities|Array|Add (LocalVariables|GetReturnActors) (.HitActor (Collision|BreakHitResult _array_element)))))
  (Class|KismetSystemLibrary|DrawDebugConeinDegrees _location _returnvalue (Variables|Default|GetSightLength) _returnvalue_2 _returnvalue_2 12 "(R=1.000000,G=1.000000,B=1.000000,A=1.000000)" 0.0 0.0)
  (return _returnactors (Utilities|Array|IsNotEmpty _returnactors)))

(fn CanSeeActor
  (params (TargetActor :type Actor%20Object%20Reference))
  (if (|TargetIsInSight TargetActor)
    (bind _outhit (Collision|LineTraceByChannel (Transformation|GetWorldLocation) (Transformation|GetActorLocation TargetActor) "TraceTypeQuery3" false 0 "ForOneFrame"))
    (return (== TargetActor (.HitActor (Collision|BreakHitResult _outhit))))
    (else
      (return false) ; ターゲットがいない
    )))

(fn IsinSight
  (params (TargetLocation :type Vector%20%28by%20ref%29))
  (return (<= (Class|KismetMathLibrary|DegAcos (Math|Vector|DotProduct (Math|Vector|GetUnitDirection(Vector) (Transformation|GetWorldLocation) TargetLocation) (Math|Vector|GetForwardVector))) (* (Variables|Default|GetSightAngle) 0.5))))